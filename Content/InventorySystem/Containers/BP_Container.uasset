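; BP_Container is an interactable world container that holds a set of items in its own inventory component.
; On BeginPlay it copies each entry of its Items array into the component's Inventory at the matching index.
; Interact toggles that inventory when the interactor is a ThirdPersonCharacter, and any actor ending overlap with the container closes it.
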(event Collision|EventActorEndOverlap
  (params (OtherActor :type Actor%20Object%20Reference))
  (Default|CloseInventory (Variables|Default|GetBP_InventoryComponent)))

(event EventInteract
  (params (Interactor :type Actor%20Object%20Reference))
  (Utilities|Casting|CastToThirdPersonCharacter Interactor)
  (Default|InventoryToggle (Variables|Default|GetBP_InventoryComponent)))

(event EventBeginPlay
  (for (_array_element _array_index) (Variables|Default|GetItems)
    (Utilities|Array|SetArrayElem (Variables|/Game/InventorySystem/BP_MenuComponent.BP_MenuComponent_C|GetInventory (Variables|Default|GetBP_InventoryComponent)) _array_index _array_element)))

(fn ConstructionScript)