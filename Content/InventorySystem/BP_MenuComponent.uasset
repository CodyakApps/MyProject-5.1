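; Inventory component that stores item slots and toggles the inventory window on the player controller's HUD canvas, switching input mode and cursor.
; PrepareInventory sizes the slot array and refreshes each item's struct from its class defaults, on BeginPlay and whenever the window opens.
; AddtoInventory fills partial stacks or empty slots, with AddtoStack passing overflow back recursively.
; EscToggle is an empty stub, its Esc menu logic left disconnected.
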(event EventBeginPlay
  (CallFunction|PrepareInventory))

(fn InventoryToggle
  (bind _returnvalue (Game|GetPlayerController 0))
  (bind _returnvalue_2 (Game|GetPlayerController 0))
  ;[1 1 1] Inventory Toggle - Open/Close
  (Variables|Default|GetInventoryWindow
    (:then
      ;;[1 1 1] If Screen already open - closes screen
      (Widget|RemovefromParent (Variables|Default|GetInventoryWindow))
      (Variables|Default|SetInventoryWindow 0)
      (Input|SetInputModeGameOnly _returnvalue)
      (Variables|/Script/Engine.PlayerController|SetbShowMouseCursor _returnvalue false))
    (:else
      (Variables|Default|GetEscWindow
        (:then
          (Widget|RemovefromParent (Variables|Default|GetEscWindow)))
        (:else
          _))
      ;;[1 1 1] If Screen not open - Opens Screen
      (CallFunction|PrepareInventory)
      (bind _returnvalue_3 (UserInterface|CreateWidget "/Game/InventorySystem/InventoryUI/BP_InventoryWindow.BP_InventoryWindow_C" 0 self))
      (Variables|Default|SetInventoryWindow _returnvalue_3)
      ;;;[1 1 1] Cast to PlayerController
      (bind _asbp_inventory_player_controller (Utilities|Casting|CastToBP_InventoryPlayerController (Game|GetPlayerController 0)))
      (bind _returnvalue_4 (Class|CanvasPanel|AddChildtoCanvas (Variables|/Game/InventorySystem/InventoryUI/BP_InventoryHUD.BP_InventoryHUD_C|GetInventory_Canvas (Variables|/Game/InventorySystem/BP_InventoryPlayerController.BP_InventoryPlayerController_C|GetHUDWidget _asbp_inventory_player_controller)) (Variables|Default|GetInventoryWindow)))
      (Class|CanvasPanelSlot|SetAutoSize _returnvalue_4 true)
      (Class|CanvasPanelSlot|SetAlignment _returnvalue_4 "(X=0.500000,Y=0.500000)")
      (Class|CanvasPanelSlot|SetAnchors _returnvalue_4 (Utilities|Struct|MakeAnchors "(X=0.500000,Y=0.500000)" "(X=0.500000,Y=0.500000)"))
      (Class|CanvasPanelSlot|SetPosition _returnvalue_4 (Variables|Default|GetPosition))
      (Input|SetInputModeGameandUI _returnvalue_2 (Variables|Default|GetInventoryWindow) "DoNotLock" true)
      (Variables|/Script/Engine.PlayerController|SetbShowMouseCursor _returnvalue_2 true))))

(fn AddtoInventory
  (params (Content_Add :type Structure%20Slots%20Structure))
  (if (.isstackable (.itemstructure Content_Add))
    (bind _stackindex (Utilities|HasPartialStack Content_Add)
      (:True
        (bind _success (CallFunction|AddtoStack Content_Add _stackindex))
        (LocalVariables|SetIsSuccessful _success))
      (:False
        (bind _success_2 (CallFunction|CreateStack Content_Add :!label _label))
        (LocalVariables|SetIsSuccessful _success_2)))
    (else
      (goto _label)))
  (return (LocalVariables|GetIsSuccessful)))

(fn PrepareInventory
  (Utilities|Array|Resize (Variables|Default|GetInventory) (Variables|Default|GetNumberofSlots))
  (for (_array_element _array_index) (Variables|Default|GetInventory)
    (if (!= (.Class (Utilities|Struct|BreakStructure_Item (.itemstructure _array_element))) 0)
      (Utilities|Array|SetArrayElem (Variables|Default|GetInventory) _array_index (Utilities|Struct|MakeStructure_Slots (.ItemStructure (Utilities|GetClassDefaults (.Class (Utilities|Struct|BreakStructure_Item (.itemstructure _array_element))))) (.quantity _array_element))))))

(fn CreateStack
  (params (Content_Add :type Structure%20Slots%20Structure))
  (bind _array_element (Utilities|Array|ForEachLoopwithBreak (Variables|Default|GetInventory) :!label _label)
    (:LoopBody
      (if (<= (.quantity _array_element) 0)
        (LocalVariables|SetHasSpace true)
        (goto _label Break)))
    (:Completed
      (if (LocalVariables|GetHasSpace)
        (bind _first_emtpy_slot (CallFunction|FindEmptySlot))
        (Utilities|Array|SetArrayElem (Variables|Default|GetInventory) _first_emtpy_slot Content_Add)
        (return (LocalVariables|GetHasSpace))
        (else
          (Development|PrintString "Inventory Full")
          (return false))))))

(fn AddtoStack
  (params (SlotStructure :type Structure%20Slots%20Structure) (SlotIndex :type Integer))
  (bind _inventory (Variables|Default|GetInventory))
  (bind _inventory_2 (Variables|Default|GetInventory))
  (bind _maxstacksize (Utilities|Struct|BreakStructure_Item (.itemstructure SlotStructure)))
  (bind _output (Utilities|Array|Get(acopy) _inventory SlotIndex))
  (bind _output_2 (Utilities|Array|Get(acopy) _inventory_2 SlotIndex))
  (bind _output_get (LocalVariables|SetCurrentQuantity (.quantity _output)))
  (if (> (+ _output_get (.Quantity (Utilities|Struct|BreakStructure_Slots SlotStructure))) (.maxstacksize (.itemstructure _output)))
    (Utilities|Array|SetArrayElem (Variables|Default|GetInventory) SlotIndex (Utilities|Struct|MakeStructure_Slots (.itemstructure SlotStructure) _maxstacksize))
    (CallFunction|AddtoInventory (Utilities|Struct|MakeStructure_Slots (.itemstructure SlotStructure) (- (.quantity SlotStructure) (- _maxstacksize (LocalVariables|GetCurrentQuantity)))))
    (else
      (Utilities|Array|SetArrayElem _inventory_2 SlotIndex (Utilities|Struct|MakeStructure_Slots (.itemstructure _output_2) (+ (.quantity _output_2) (.quantity SlotStructure))))))
  (return true))

(fn EscToggle
  ;[1 1 1] Esc Menu Toggle - Open/Close
)

(fn CloseInventory
  (bind _returnvalue (Game|GetPlayerController 0))
  (Variables|Default|GetInventoryWindow
    (:then
      (Widget|RemovefromParent (Variables|Default|GetInventoryWindow))
      (Variables|Default|SetInventoryWindow 0)
      (Input|SetInputModeGameOnly _returnvalue)
      (Variables|/Script/Engine.PlayerController|SetbShowMouseCursor _returnvalue false))
    (:else)))

(fn FindEmptySlot
  (bind (_array_element _array_index) (Utilities|Array|ForEachLoopwithBreak (Variables|Default|GetInventory) :!label _label)
    (:LoopBody
      (if (== (.quantity _array_element) 0)
        (Variables|Default|SetSlotIndex _array_index)
        (goto _label Break)))
    (:Completed
      (return (Variables|Default|GetSlotIndex)))))