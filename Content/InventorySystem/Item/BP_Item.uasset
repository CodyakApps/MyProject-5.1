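; BP_Item is an inventory item actor with a UseItem function that simply returns true.
; On BeginPlay it stores itself in its ItemInfo struct and binds PickupItemEvent to the player character's PickupItem dispatcher.
; The pickup, range check and server removal events do nothing.
; Logic for adding to inventory, destroying or hiding the actor, and refreshing the HUD is left disconnected.
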(event Custom|PickupItemEvent
  (if (and (stale EventRangeCheck InRange) (Collision|GetActorEnableCollision))
    _))

(event EventRemoveObjectServer)

(event EventBeginPlay
  (Utilities|Struct|SetmembersinInventoryStruct (Variables|Default|GetItemInfo) self)
  (bind _asthird_person_character (Utilities|Casting|CastToThirdPersonCharacter (Game|GetPlayerCharacter 0)))
  (bind _output_get (Variables|Default|SetCharacterReference _asthird_person_character))
  (EventDispatchers|BindEventtoPickupItem _output_get (delegate Custom|PickupItemEvent)))

(event EventRangeCheck
  (params (InRange :type Boolean)))

(fn ConstructionScript)

(fn UseItem
  (return true))